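; Simon memory-game pawn that wires four colored buttons and a start button to game logic defined outside these graphs.
; BeginPlay registers the buttons and binds hover to cursor changes.
; Clicks and touches feed colored buttons into the player sequence, while the start button pushes and starts the game.
; Turn and game-over events only print messages; the input-gated PlayButton function is not called here.
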(event Custom|CustomEvent_0
  (params (FingerIndex :type ETouchIndex%20Enum :default "Touch1") (TouchedComponent :type Primitive%20Component%20Object%20Reference))
  ;[1 1 1] Setup Simon Buttons Events
  (bind _assimon_button (Utilities|Casting|CastToSimonButton TouchedComponent))
  (Class|PlayerPawn|AddtoPlayerSequence _assimon_button))

(event Custom|CustomEvent_1
  (params (TouchedComponent :type Primitive%20Component%20Object%20Reference) (ButtonPressed :type Key%20Structure))
  ;[1 1 1] Setup Start Button Events
  (Class|ButtonStaticMesh|Push (Variables|Default|GetStartButton))
  (Class|PlayerPawn|StartGame))

(event Custom|OnEndCursorOver_Event_0
  (params (TouchedComponent :type Primitive%20Component%20Object%20Reference))
  ;[1 1 1] Setup Simon Buttons Events
  (Class|PlayerPawn|ShowDefaultCursor))

(event Custom|CustomEvent_2
  (params (FingerIndex :type ETouchIndex%20Enum :default "Touch1") (TouchedComponent :type Primitive%20Component%20Object%20Reference))
  ;[1 1 1] Setup Start Button Events
  (Class|ButtonStaticMesh|Push (Variables|Default|GetStartButton))
  (Class|PlayerPawn|StartGame))

(event Custom|OnClicked_Event_0
  (params (TouchedComponent :type Primitive%20Component%20Object%20Reference) (ButtonPressed :type Key%20Structure))
  ;[1 1 1] Setup Simon Buttons Events
  (bind _assimon_button (Utilities|Casting|CastToSimonButton TouchedComponent))
  (Class|PlayerPawn|AddtoPlayerSequence _assimon_button))

(event Custom|OnBeginCursorOver_Event_0
  (params (TouchedComponent :type Primitive%20Component%20Object%20Reference))
  ;[1 1 1] Setup Simon Buttons Events
  (Class|PlayerPawn|ShowHandCursor))

(event EventBeginPlay
  (bind _startbutton (Variables|Default|GetStartButton))
  ;[1 1 1] Init Buttons Array
  (bind _output_get (Variables|Default|SetButtonsArray (Utilities|Array|MakeArray (Variables|Default|GetRedButton) (Variables|Default|GetBlueButton) (Variables|Default|GetGreenButton) (Variables|Default|GetYellowButton))))
  (for _array_element _output_get
    ;[1 1 1] Setup Simon Buttons Events
    (EventDispatchers|AssignOnBeginCursorOver _array_element (delegate Custom|OnBeginCursorOver_Event_0))
    (EventDispatchers|AssignOnEndCursorOver _array_element (delegate Custom|OnEndCursorOver_Event_0))
    (EventDispatchers|AssignOnClicked _array_element (delegate Custom|OnClicked_Event_0))
    (EventDispatchers|BindEventtoOnInputTouchEnter _array_element (delegate Custom|CustomEvent_0)))
  (Class|PlayerPawn|Initialise _output_get)
  ;[1 1 1] Setup Start Button Events
  (EventDispatchers|BindEventtoOnBeginCursorOver _startbutton (delegate Custom|OnBeginCursorOver_Event_0))
  (EventDispatchers|BindEventtoOnEndCursorOver _startbutton (delegate Custom|OnEndCursorOver_Event_0))
  (EventDispatchers|BindEventtoOnClicked _startbutton (delegate Custom|CustomEvent_1))
  (EventDispatchers|BindEventtoOnInputTouchEnter _startbutton (delegate Custom|CustomEvent_2)))

(event EventOnWrongButton
  (params (TurnCount :type Float%20%28single-precision%29))
  ;[1 1 1] Game Over
  (Development|PrintString "Game Over"))

(event EventOnChallangeTurn
  ;[1 1 1] Challange Turn
  (Development|PrintString "Challange Turn"))

(event EventOnPlayerTurn
  ;[1 1 1] Player Turn
  (Development|PrintString "Player Turn"))

(event EventOnTimeIsOver
  (params (TurnCount :type Float%20%28single-precision%29))
  ;[1 1 1] Game Over
  (Development|PrintString "Game Over"))

(fn ConstructionScript)

(fn PlayButton
  (params (TouchedComp :type Primitive%20Component%20Object%20Reference))
  (if (Variables|Default|GetIsInputEnabled)
    (bind _assimon_button (Utilities|Casting|CastToSimonButton TouchedComp))
    (Class|SimonButton|Play _assimon_button)
    (Class|PlayerPawn|AddtoPlayerSequence _assimon_button)))